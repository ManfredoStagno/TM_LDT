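; MovingPlatform2 is a platform Blueprint that can move its static mesh along a spline.
; When IsMovingPlatform is set at BeginPlay, the MovePlatform timeline plays, and its TravelDistance track, scaled by spline length, gives the mesh's world location without sweeping.
; A yaw-alignment step from the spline's rotation exists but is unconnected, so it never runs.
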(event `self.ReceiveBeginPlay`
  (if (`self.IsMovingPlatform`)
    (bind (_direction _traveldistance) (`Timeline|MovePlatform`)
      (:`Update`
        (`SceneComponent.K2_SetWorldLocation` (`self.StaticMesh`) (`SplineComponent.GetLocationAtDistanceAlongSpline` (`self.Spline`) (* _traveldistance (`SplineComponent.GetSplineLength` (`self.Spline`))) "World") false false)))))

(fn `UserConstructionScript`)