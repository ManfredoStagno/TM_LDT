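; Damager is a hazard that damages overlapping BP_Base actors and can optionally move as a platform.
; When IsMovingPlatform is set, a timeline started at BeginPlay moves the static mesh along a spline without sweeping.
; Overlapping the Box calls TakeDamage on the BP_Base unless it is invulnerable.
; Spline-based rotation logic is present but disconnected, so it never runs.
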(event `self.ReceiveBeginPlay`
  (if (`self.IsMovingPlatform`)
    (bind (_direction _traveldistance) (`Timeline|MovePlatform`)
      (:`Update`
        (`SceneComponent.K2_SetWorldLocation` (`self.StaticMesh`) (`SplineComponent.GetLocationAtDistanceAlongSpline` (`self.Spline`) (* _traveldistance (`SplineComponent.GetSplineLength` (`self.Spline`))) "World") false false)))))

(event `self.StaticMesh.OnComponentBeginOverlap`
  (params (OverlappedComponent :type "PrimitiveComponent Object Reference") (OtherActor :type "Actor Object Reference") (OtherComp :type "PrimitiveComponent Object Reference") (OtherBodyIndex :type Integer) (bFromSweep :type Boolean) (SweepResult :type "HitResult Structure (by ref)")))

(event `self.Box.OnComponentBeginOverlap`
  (params (OverlappedComponent :type "PrimitiveComponent Object Reference") (OtherActor :type "Actor Object Reference") (OtherComp :type "PrimitiveComponent Object Reference") (OtherBodyIndex :type Integer) (bFromSweep :type Boolean) (SweepResult :type "HitResult Structure (by ref)"))
  (bind _asbp_base (cast `/Game/Blueprints/BP_Base` OtherActor))
  (if (not (`/Game/Blueprints/BP_Base.IsInvulnerable` _asbp_base))
    (`/Game/Blueprints/BP_Base.TakeDamage` _asbp_base)))

(fn `UserConstructionScript`)