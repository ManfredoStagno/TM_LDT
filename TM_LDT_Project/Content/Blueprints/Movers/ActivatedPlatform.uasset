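; Moving platform that travels along a spline when a BP_Base actor enters its trigger box.
; The overlap plays the MovePlatform timeline if IsMovingPlatform is set.
; Each update scales TravelDistance by spline length to set the static mesh's world location, without sweeping.
; A node for setting mesh yaw from the spline is unconnected, so the platform does not rotate.
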(event `self.Box.OnComponentBeginOverlap`
  (params (OverlappedComponent :type "PrimitiveComponent Object Reference") (OtherActor :type "Actor Object Reference") (OtherComp :type "PrimitiveComponent Object Reference") (OtherBodyIndex :type Integer) (bFromSweep :type Boolean) (SweepResult :type "HitResult Structure (by ref)"))
  (cast `/Game/Blueprints/BP_Base` OtherActor)
  (if (`self.IsMovingPlatform`)
    (bind (_direction _traveldistance) (`Timeline|MovePlatform`)
      (:`Update`
        (`SceneComponent.K2_SetWorldLocation` (`self.StaticMesh`) (`SplineComponent.GetLocationAtDistanceAlongSpline` (`self.Spline`) (* _traveldistance (`SplineComponent.GetSplineLength` (`self.Spline`))) "World") false false)))))

(fn `UserConstructionScript`)