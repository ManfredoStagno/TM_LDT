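; MovableCube is a pushable cube that only simulates physics while a BP_Base actor is in one of its trigger volumes.
; Separate X-axis and Y-axis collision components share the same logic: begin overlap enables physics on the Cube and sets IsPushing on the BP_Base.
; End overlap from either volume reverses both, without checking whether the other volume is still overlapped.
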(event `self.Y Axis collision.OnComponentBeginOverlap`
  (params (OverlappedComponent :type "PrimitiveComponent Object Reference") (OtherActor :type "Actor Object Reference") (OtherComp :type "PrimitiveComponent Object Reference") (OtherBodyIndex :type Integer) (bFromSweep :type Boolean) (SweepResult :type "HitResult Structure (by ref)"))
  (bind _asbp_base (cast `/Game/Blueprints/BP_Base` OtherActor))
  (`PrimitiveComponent.SetSimulatePhysics` (`self.Cube`) true)
  (set `/Game/Blueprints/BP_Base.IsPushing` true _asbp_base))

(event `self.Y Axis collision.OnComponentEndOverlap`
  (params (OverlappedComponent :type "PrimitiveComponent Object Reference") (OtherActor :type "Actor Object Reference") (OtherComp :type "PrimitiveComponent Object Reference") (OtherBodyIndex :type Integer))
  (bind _asbp_base (cast `/Game/Blueprints/BP_Base` OtherActor))
  (`PrimitiveComponent.SetSimulatePhysics` (`self.Cube`) false)
  (set `/Game/Blueprints/BP_Base.IsPushing` false _asbp_base))

(event `self.X Axis collision.OnComponentBeginOverlap`
  (params (OverlappedComponent :type "PrimitiveComponent Object Reference") (OtherActor :type "Actor Object Reference") (OtherComp :type "PrimitiveComponent Object Reference") (OtherBodyIndex :type Integer) (bFromSweep :type Boolean) (SweepResult :type "HitResult Structure (by ref)"))
  (bind _asbp_base (cast `/Game/Blueprints/BP_Base` OtherActor))
  (`PrimitiveComponent.SetSimulatePhysics` (`self.Cube`) true)
  (set `/Game/Blueprints/BP_Base.IsPushing` true _asbp_base))

(event `self.X Axis collision.OnComponentEndOverlap`
  (params (OverlappedComponent :type "PrimitiveComponent Object Reference") (OtherActor :type "Actor Object Reference") (OtherComp :type "PrimitiveComponent Object Reference") (OtherBodyIndex :type Integer))
  (bind _asbp_base (cast `/Game/Blueprints/BP_Base` OtherActor))
  (`PrimitiveComponent.SetSimulatePhysics` (`self.Cube`) false)
  (set `/Game/Blueprints/BP_Base.IsPushing` false _asbp_base))

(fn `UserConstructionScript`)