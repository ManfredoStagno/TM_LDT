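; Game mode that handles player respawning, checkpoints and coin, gem and key tallies.
; On BeginPlay and after each respawn, it binds OnDie to the BP_Base character's destruction and saves that character's transform as the checkpoint.
; OnDie waits briefly, spawns and possesses a new BP_Base at the saved transform, then rebinds through Respawn.
; Counter functions increment their totals and print them on screen, though GemCount labels its total "Coins".
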(event `Respawn`
  (bind _asbp_base (cast `/Game/Blueprints/BP_Base` (`GameplayStatics.GetPlayerCharacter` 0) :!label _label))
  (add `self.OnDestroyed` _asbp_base (delegate `OnDie`))
  (`self.UpdateCheckpoint`))

(event `self.ReceiveBeginPlay`
  (goto _label))

(event `OnDie` :!signature `self.OnDestroyed`
  (params (DestroyedActor :type "Actor Object Reference"))
  (`KismetSystemLibrary.Delay` 2.0)
  (bind _returnvalue (`|SpawnActorFromClass` "/Game/Blueprints/BP_Base.BP_Base_C" (`self.SpawnTransform`) "Undefined" "OverrideRootScale" null null))
  (`Controller.Possess` (`GameplayStatics.GetPlayerController` 0) _returnvalue)
  (`self.Respawn`))

(fn `CoinCount`
  (bind _result (`/Engine/EditorBlueprintResources/StandardMacros.IncrementInt` (`self.Coins`))
    (:`  `
      (bind _output_get (set `self.Coins` _result))
      (`KismetSystemLibrary.PrintString` (`KismetStringLibrary.Conv_IntToString` _output_get) true true (struct :`R` 1.0 :`G` 0.91268 :`B` 0.028845 :`A` 1.0))
      (`KismetSystemLibrary.PrintString` "Coins" true true (struct :`R` 1.0 :`G` 0.913099 :`B` 0.028426 :`A` 1.0)))))

(fn `GemCount`
  (bind _result (`/Engine/EditorBlueprintResources/StandardMacros.IncrementInt` (`self.Gems`))
    (:`  `
      (bind _output_get (set `self.Gems` _result))
      (`KismetSystemLibrary.PrintString` (`KismetStringLibrary.Conv_IntToString` _output_get) true true (struct :`R` 1.0 :`B` 0.940751 :`A` 1.0))
      (`KismetSystemLibrary.PrintString` "Coins" true true (struct :`R` 0.957613 :`B` 1.0 :`A` 1.0)))))

(fn `KeyCount`
  (bind _result (`/Engine/EditorBlueprintResources/StandardMacros.IncrementInt` (`self.Keys`))
    (:`  `
      (bind _output_get (set `self.Keys` _result))
      (`KismetSystemLibrary.PrintString` (`KismetStringLibrary.Conv_IntToString` _output_get) true true (struct :`G` 1.0 :`B` 0.029682 :`A` 1.0))
      (`KismetSystemLibrary.PrintString` "Keys" true true (struct :`R` 0.074615 :`G` 1.0 :`B` 0.092892 :`A` 1.0)))))

(fn `UpdateCheckpoint`
  (bind _asbp_base (cast `/Game/Blueprints/BP_Base` (`GameplayStatics.GetPlayerCharacter` 0)))
  (set `self.SpawnTransform` (`self.GetTransform` _asbp_base))
  (`KismetSystemLibrary.PrintString` "Checkpint Updated"))

(fn `UserConstructionScript`)