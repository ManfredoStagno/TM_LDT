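; Trigger-driven camera actor that takes over the player's view in a zone, either from a fixed position or following the player.
; Start and end trigger overlaps by BP_Base blend the view target to this actor and back to the character.
; While it is the view target, Tick either turns the camera toward the player or moves the spring arm, masked per axis by TrackPlayer, and optionally rotates it to face them.
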(event `self.ReceiveBeginPlay`
  ;[1 1 1] Comment
)

(event `self.StartTrigger.OnComponentBeginOverlap`
  (params (OverlappedComponent :type "PrimitiveComponent Object Reference") (OtherActor :type "Actor Object Reference") (OtherComp :type "PrimitiveComponent Object Reference") (OtherBodyIndex :type Integer) (bFromSweep :type Boolean) (SweepResult :type "HitResult Structure (by ref)"))
  (cast `/Game/Blueprints/BP_Base` OtherActor)
  (`PlayerController.SetViewTargetWithBlend` (`GameplayStatics.GetPlayerController` 0) self (`self.BlendTime`) "VTBlend_Linear" 0.0 false)
  (`/Engine/EditorBlueprintResources/StandardMacros.DoOnce` false
    (:`Completed`
      (set `self.Offset` (- (`self.K2_GetActorLocation`) (`SceneComponent.K2_GetComponentLocation` (`self.SpringArm`)))))))

(event `self.EndTrigger.OnComponentBeginOverlap`
  (params (OverlappedComponent :type "PrimitiveComponent Object Reference") (OtherActor :type "Actor Object Reference") (OtherComp :type "PrimitiveComponent Object Reference") (OtherBodyIndex :type Integer) (bFromSweep :type Boolean) (SweepResult :type "HitResult Structure (by ref)"))
  (bind _asbp_base (cast `/Game/Blueprints/BP_Base` OtherActor))
  (`PlayerController.SetViewTargetWithBlend` (`GameplayStatics.GetPlayerController` 0) _asbp_base (`self.BlendTime`) "VTBlend_Linear" 0.0 false))

(event `self.ReceiveTick`
  (params (DeltaSeconds :type "Float (single-precision)"))
  (if (== (`Controller.GetViewTarget` (`GameplayStatics.GetPlayerController` 0)) self)
    (if (`self.IsStationary`)
      (bind _rotation (`self.StationaryRotation` DeltaSeconds))
      (`SceneComponent.K2_SetWorldRotation` (`self.Camera`) _rotation false false)
      (else
        (bind _vector (`self.FollowMovement` DeltaSeconds))
        (`SceneComponent.K2_SetWorldLocation` (`self.SpringArm`) _vector false false)
        (if (`self.IsRotating`)
          (bind _rotation_2 (`self.MovingRotation` DeltaSeconds))
          (`SceneComponent.K2_SetWorldRotation` (`self.SpringArm`) _rotation_2 false false)
          (cast `/Game/Blueprints/BP_Base` (`GameplayStatics.GetPlayerCharacter` 0)))))))

(fn `FollowMovement`
  (params (DeltaTime :type "Float (double-precision)"))
  (returns (Vector :type "Vector Structure"))
  (bind _trackplayer (`self.TrackPlayer`))
  (bind _returnvalue (- (`self.K2_GetActorLocation`) (`self.Offset`)))
  (return (`KismetMathLibrary.VInterpTo` _returnvalue (+ (* (`self.K2_GetActorLocation` (`GameplayStatics.GetPlayerCharacter` 0)) _trackplayer) (* _returnvalue (- (1.0 1.0 1.0) _trackplayer))) DeltaTime)))

(fn `MovingRotation`
  (params (Delta :type "Float (double-precision)"))
  (returns (Rotation :type "Rotator Structure"))
  (return (`KismetMathLibrary.FindLookAtRotation` (`SceneComponent.K2_GetComponentLocation` (`self.SpringArm`)) (`self.K2_GetActorLocation` (`GameplayStatics.GetPlayerCharacter` 0)))))

(fn `StationaryRotation`
  (params (Delta :type "Float (double-precision)"))
  (returns (Rotation :type "Rotator Structure"))
  (return (`KismetMathLibrary.FindLookAtRotation` (`SceneComponent.K2_GetComponentLocation` (`self.Camera`)) (`self.K2_GetActorLocation` (`GameplayStatics.GetPlayerCharacter` 0)))))

(fn `UserConstructionScript`)