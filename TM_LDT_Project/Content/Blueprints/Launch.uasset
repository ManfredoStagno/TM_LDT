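; Launch Blueprint that bounces the player character upward while it is inside a trigger sphere, like a jump pad.
; Overlap events on Sphere2 set an inside flag when a BP_Base actor enters or leaves.
; Each tick while the flag is set, it checks whether the player character is falling, then stops its jump and launches it upward, overriding vertical velocity.
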(event `self.Sphere2.OnComponentBeginOverlap`
  (params (OverlappedComponent :type "PrimitiveComponent Object Reference") (OtherActor :type "Actor Object Reference") (OtherComp :type "PrimitiveComponent Object Reference") (OtherBodyIndex :type Integer) (bFromSweep :type Boolean) (SweepResult :type "HitResult Structure (by ref)"))
  (cast `/Game/Blueprints/BP_Base` OtherActor)
  (set `self.IsInsideSphere` true))

(event `self.Sphere2.OnComponentEndOverlap`
  (params (OverlappedComponent :type "PrimitiveComponent Object Reference") (OtherActor :type "Actor Object Reference") (OtherComp :type "PrimitiveComponent Object Reference") (OtherBodyIndex :type Integer))
  (cast `/Game/Blueprints/BP_Base` OtherActor)
  (set `self.IsInsideSphere` false))

(event `self.ReceiveTick`
  (params (DeltaSeconds :type "Float (single-precision)"))
  (if (`self.IsInsideSphere`)
    (bind _asbp_base (cast `/Game/Blueprints/BP_Base` (`GameplayStatics.GetPlayerCharacter` 0)))
    (bind (_returnvalue_x _returnvalue_y _returnvalue_z) (`KismetMathLibrary.BreakVector` (`self.GetVelocity` _asbp_base)))
    (if (< _returnvalue_z 0.0)
      (`Character.StopJumping` _asbp_base)
      (`Character.LaunchCharacter` _asbp_base (0.0 0.0 1500.0) false true))))

(fn `UserConstructionScript`)