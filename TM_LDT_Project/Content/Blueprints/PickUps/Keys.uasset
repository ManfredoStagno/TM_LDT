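; Key pickup that the BP_Base actor collects by overlapping its box, which calls KeyCount on MyGameMode and destroys the key.
; Every tick it spins in yaw and plays the Floating timeline, whose track value is added to the current Z position to move it vertically.
; A pickup sound node exists but is not wired, so it never plays.
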(event `self.Box.OnComponentBeginOverlap`
  (params (OverlappedComponent :type "PrimitiveComponent Object Reference") (OtherActor :type "Actor Object Reference") (OtherComp :type "PrimitiveComponent Object Reference") (OtherBodyIndex :type Integer) (bFromSweep :type Boolean) (SweepResult :type "HitResult Structure (by ref)"))
  (cast `/Game/Blueprints/BP_Base` OtherActor)
  (bind _asmy_game_mode (cast `/Game/Blueprints/MyGameMode` (`GameplayStatics.GetGameMode`)))
  (`/Game/Blueprints/MyGameMode.KeyCount` _asmy_game_mode)
  (`self.K2_DestroyActor`))

(event `self.ReceiveTick`
  (params (DeltaSeconds :type "Float (single-precision)"))
  (`self.K2_AddActorLocalRotation` (struct :`Yaw` 1.0))
  (bind (_direction _newtrack_1) (`Timeline|Floating`)
    (:`Update`
      (`self.K2_SetActorLocation` (+ (`self.K2_GetActorLocation`) (`KismetMathLibrary.MakeVector` 0.0 0.0 _newtrack_1))))))

(fn `UserConstructionScript`)